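; VR player pawn with motion-controller teleporting and pool cue interaction.
; While right Button1 is held, a controller line trace finds a navmesh-projected point shown by a debug cylinder; release teleports there, offset by camera position, if the surface was near-flat.
; Each trigger messages the first overlapping BP_PoolCue with its hold state, though both pass the right controller as hand.
; Left Button1 sends that cue an activate message.
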(event EventTick
  (params (DeltaSeconds :type Float%20%28single-precision%29))
  (bind _motioncontroller_r (Variables|Default|GetMotionController_R))
  (if (Variables|Default|GetbTriggerHeld)
    (CallFunction|GetTPDestination (Transformation|GetWorldLocation _motioncontroller_r) (Math|Vector|GetForwardVector _motioncontroller_r))))

(event Input|ActionEvents|InputActionMotionController(R)Button1
  (params (Key :type Key%20Structure :default "None"))
  (:Pressed
    (Variables|Default|SetbTriggerHeld true))
  (:Released
    (Variables|Default|SetbTriggerHeld false)
    (if (Variables|Default|GetbTeleport)
      (CallFunction|TeleporttoDestination (Variables|Default|GetTeleportLoc)))))

(event Input|ActionEvents|InputActionMotionController(R)Trigger
  (params (Key :type Key%20Structure :default "None"))
  (:Pressed
    (Variables|Default|SetbHoldingR true)
    (Class|IInteractable|Interact(Message) (Utilities|Array|Get(acopy) (Collision|GetOverlappingActors (Variables|Default|GetBoxR) "/Game/Blueprints/Interactable/BP_PoolCue.BP_PoolCue_C" :!class /Script/Engine.PrimitiveComponent)) (Variables|Default|GetMotionController_R) (Variables|Default|GetbHoldingR) :!label _label))
  (:Released
    (Variables|Default|SetbHoldingR false)
    (goto _label)))

(event Input|ActionEvents|InputActionMotionController(L)Trigger
  (params (Key :type Key%20Structure :default "None"))
  (:Pressed
    (Variables|Default|SetbHoldingL true)
    (Class|IInteractable|Interact(Message) (Utilities|Array|Get(acopy) (Collision|GetOverlappingActors (Variables|Default|GetBoxL) "/Game/Blueprints/Interactable/BP_PoolCue.BP_PoolCue_C" :!class /Script/Engine.PrimitiveComponent)) (Variables|Default|GetMotionController_R) (Variables|Default|GetbHoldingL) :!label _label))
  (:Released
    (Variables|Default|SetbHoldingL false)
    (goto _label)))

(event Input|ActionEvents|InputActionMotionController(L)Button1
  (params (Key :type Key%20Structure :default "None"))
  (:Pressed
    (Class|IInteractable|Activate(Message) (Utilities|Array|Get(acopy) (Collision|GetOverlappingActors (Variables|Default|GetBoxL) "/Game/Blueprints/Interactable/BP_PoolCue.BP_PoolCue_C" :!class /Script/Engine.PrimitiveComponent)))))

(fn ConstructionScript)

(fn GetTPDestination
  (params (Position :type Vector) (ForwardVector :type Vector))
  (bind _outhit (Collision|LineTraceByChannel Position (+ Position (* ForwardVector 1e+04)) "TraceTypeQuery1" false 0 "None"))
  (Variables|Default|SetbTeleport (> (Math|Vector|DotProduct (.Normal (Collision|BreakHitResult _outhit)) "0, 0,1.000000") 0.9))
  (if true
    (bind _output_get (Variables|Default|SetTeleportLoc (.ProjectedLocation (AI|Navigation|ProjectPointtoNavigation (.Location (Collision|BreakHitResult _outhit)) 0 0 "0, 0, 0"))))
    (Class|KismetSystemLibrary|DrawDebugCylinder _output_get (+ _output_get (* (.Normal (Collision|BreakHitResult _outhit)) 1e+01)) 1e+02 12 "(R=0.035597,G=1.000000,B=0.039146,A=1.000000)" 0.0 2.0)))

(fn TeleporttoDestination
  (params (Location :type Vector))
  (bind _vr_camera (Variables|Default|GetVR_Camera))
  (bind _relativelocation (Variables|/Script/Engine.SceneComponent|GetRelativeLocation _vr_camera))
  (Transformation|SetActorLocation (+ Location (Math|Vector|MakeVector (.x _relativelocation) (.y _relativelocation) 0.0)) false false))